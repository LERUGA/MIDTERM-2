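; BP_MazeCell is a modular maze cell whose construction script sizes a floor and adds optional walls from grid size and wall height.
; Optional ceiling and point light are built inside a loop over Lose widgets, because the branch condition is fixed true.
; At BeginPlay it binds to the game mode's game-over dispatcher to turn NewVar's light red.
; NewVar is only assigned in the unreachable false branch.
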(event `self.ReceiveBeginPlay`
  (bind _asgame_mode (cast `/Game/NewFolder1/GameMode` (`GameplayStatics.GetGameMode`)))
  (bind _output_get (set `self.As GM 901` _asgame_mode))
  (add `/Game/NewFolder1/GameMode.GameOverDP` _output_get (delegate `CustomEvent`)))

(event `CustomEvent`
  (`LightComponent.SetLightColor` (`self.NewVar`) (struct :`R` 1.0 :`B` 0.023381 :`A` 1.0) true))

(fn `UserConstructionScript`
  (locals (`Wall Length` :type "Float (double-precision)") (`Wall Thickness` :type "Float (double-precision)"))
  (bind _gridsize (`self.GridSize`))
  (bind _wall_length (`local.Wall Length`))
  (bind _wall_length_2 (`local.Wall Length`))
  (bind _wall_length_3 (`local.Wall Length`))
  (bind _returnvalue (* (`local.Wall Length`) 0.5))
  (bind _returnvalue_2 (* (`local.Wall Length`) 0.5))
  (set `local.Wall Length` _gridsize)
  (set `local.Wall Thickness` (* _gridsize 0.1))
  (`SceneComponent.SetRelativeScale3D` (`self.Floor`) (`self.SizeToCubeScale` (`KismetMathLibrary.MakeVector` _wall_length _wall_length (`local.Wall Thickness`))))
  (if (`self.WestWall`)
    (`AddComponent|NODE_AddStaticMeshComponent-4` :`RelativeTransform` (`KismetMathLibrary.MakeTransform` (0.0 0.0 0.0) (struct) (`self.SizeToCubeScale` (`KismetMathLibrary.MakeVector` (`local.Wall Length`) (`local.Wall Thickness`) (`self.WallHeight`))))))
  (if (`self.SouthWall`)
    (`AddComponent|NODE_AddStaticMeshComponent-5` :`RelativeTransform` (`KismetMathLibrary.MakeTransform` (0.0 0.0 0.0) (struct) (`self.SizeToCubeScale` (`KismetMathLibrary.MakeVector` (`local.Wall Thickness`) (`local.Wall Length`) (`self.WallHeight`))))))
  (if (`self.NorthWall`)
    (`AddComponent|NODE_AddStaticMeshComponent-6` :`RelativeTransform` (`KismetMathLibrary.MakeTransform` (`KismetMathLibrary.MakeVector` (- (`local.Wall Length`) (`local.Wall Thickness`))) (struct) (`self.SizeToCubeScale` (`KismetMathLibrary.MakeVector` (`local.Wall Thickness`) (`local.Wall Length`) (`self.WallHeight`))))))
  (if (`self.EastWall`)
    (`AddComponent|NODE_AddStaticMeshComponent-7` :`RelativeTransform` (`KismetMathLibrary.MakeTransform` (`KismetMathLibrary.MakeVector` 0.0 (- (`local.Wall Length`) (`local.Wall Thickness`))) (struct) (`self.SizeToCubeScale` (`KismetMathLibrary.MakeVector` (`local.Wall Length`) (`local.Wall Thickness`) (`self.WallHeight`))))))
  (if true
    (bind _foundwidgets (`WidgetBlueprintLibrary.GetAllWidgetsOfClass` "/Game/NewFolder1/Lose.Lose_C"))
    (for _ _foundwidgets
      (if (`self.Ceiling`)
        (`AddComponent|NODE_AddStaticMeshComponent-9` :`RelativeTransform` (`KismetMathLibrary.MakeTransform` (`KismetMathLibrary.MakeVector` 0.0 0.0 (`self.WallHeight`)) (struct) (`self.SizeToCubeScale` (`KismetMathLibrary.MakeVector` _wall_length_2 _wall_length_2 (`local.Wall Thickness`)))))
        (if (> (`self.LightIntensity`) 0.0)
          (bind _returnvalue_3 (`AddComponent|NODE_AddPointLightComponent-1` :`RelativeTransform` (`KismetMathLibrary.MakeTransform` (`KismetMathLibrary.MakeVector` _returnvalue _returnvalue (* (`self.WallHeight`) 0.9)))))
          (`LightComponent.SetLightColor` _returnvalue_3 (`self.LightColor2`) true)
          (`LightComponent.SetIntensity` _returnvalue_3 (`self.LightIntensity`)))))
    (elif (`self.Ceiling`)
      (`AddComponent|NODE_AddStaticMeshComponent-8` :`RelativeTransform` (`KismetMathLibrary.MakeTransform` (`KismetMathLibrary.MakeVector` 0.0 0.0 (`self.WallHeight`)) (struct) (`self.SizeToCubeScale` (`KismetMathLibrary.MakeVector` _wall_length_3 _wall_length_3 (`local.Wall Thickness`)))))
      (if (> (`self.LightIntensity`) 0.0)
        (bind _returnvalue_4 (`AddComponent|NODE_AddPointLightComponent-0` :`RelativeTransform` (`KismetMathLibrary.MakeTransform` (`KismetMathLibrary.MakeVector` _returnvalue_2 _returnvalue_2 (* (`self.WallHeight`) 0.9)))))
        (bind _output_get (set `self.NewVar` _returnvalue_4))
        (`LightComponent.SetLightColor` _output_get (`self.LightColor`) true)
        (`LightComponent.SetIntensity` _output_get (`self.LightIntensity`))))))